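; Game mode for an Arkanoid-style game that tracks score and lives and spawns balls at the player platform.
; After a short delay at start, it caches the blocks, spawns a ball and binds scoring to the box spawner's block-destroyed event.
; Score comes from a block-type lookup map.
; The kill-zone handler deducts a life and respawns only when no more than one ball exists, with no game-over check.
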(event `self.ReceiveBeginPlay`
  (`KismetSystemLibrary.Delay` 1.5)
  (bind _outactors (`GameplayStatics.GetAllActorsOfClass` "/Game/Actors/BP_MasterBox.BP_MasterBox_C"))
  (bind _output_get (set `self.Blocks` _outactors))
  (`KismetSystemLibrary.PrintString` (`KismetStringLibrary.Conv_IntToString` (`KismetArrayLibrary.Array_Length` _output_get)))
  (`self.AddNewBall`)
  (bind _returnvalue (`GameplayStatics.GetActorOfClass` "/Game/Actors/BP_BoxSpawner.BP_BoxSpawner_C"))
  (bind _output_get_2 (set `self.BoxSpawner` _returnvalue))
  (`/Engine/EditorBlueprintResources/StandardMacros.IsValid` _output_get_2
    (:`Is Valid`
      (add `/Game/Actors/BP_BoxSpawner.BlockDestroyed` (`self.BoxSpawner`) (delegate `AddScore`)))))

(event `AddScore`
  (params (BlockType :type "/Game/Blueprints/BlockTypes Enum" :default "NewEnumerator0"))
  (bind (_value _returnvalue) (`BlueprintMapLibrary.Map_Find` (`self.ScoreForBlock`) BlockType))
  (if _returnvalue
    (bind _output_get (set `self.Score` (+ _value (`self.Score`))))
    (`KismetSystemLibrary.PrintString` (`KismetStringLibrary.BuildString_Int` "Score: " "" _output_get) true true (struct :`R` 1.0 :`B` 0.120664 :`A` 1.0) 7.0)
    (else
      (`KismetSystemLibrary.PrintString` "Error: There is no such block type in type map" true true (struct :`R` 1.0 :`B` 0.10567 :`A` 1.0)))))

(event `BallInKillZone`
  (bind _outactors (`GameplayStatics.GetAllActorsOfClass` "/Game/Actors/BP_Ball.BP_Ball_C"))
  (if (not (> (`KismetArrayLibrary.Array_Length` _outactors) 1))
    (bind _result (`/Engine/EditorBlueprintResources/StandardMacros.DecrementInt` (`self.Lifes`))
      (:`  `
        (`KismetSystemLibrary.PrintString` (`KismetStringLibrary.Conv_IntToString` _result) true true (struct :`G` 0.66 :`B` 1.0 :`A` 1.0) 5.0)
        (`self.AddNewBall`)))))

(fn `AddNewBall`
  (bind _returnvalue (`GameplayStatics.GetActorOfClass` "/Game/Actors/BP_PlayerPlatform.BP_PlayerPlatform_C"))
  (bind _returnvalue_2 (`|SpawnActorFromClass` "/Game/Actors/BP_Ball.BP_Ball_C" (`SceneComponent.K2_GetComponentToWorld` (`/Game/Actors/BP_PlayerPlatform.BallSpawnPoint` _returnvalue)) "AlwaysSpawn" "MultiplyWithRoot" null null))
  (add `/Game/Actors/BP_Ball.BallKill` _returnvalue_2 (`|CreateDelegate` :!event `BallInKillZone`)))

(fn `UserConstructionScript`)