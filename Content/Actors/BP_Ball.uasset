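; BP_Ball is a bouncing ball actor that travels in a straight line until it hits something or enters a kill volume.
; Each Tick it does a swept offset along Direction scaled by Speed and delta time, reflecting Direction off the hit normal on a blocking hit, without physics simulation.
; Overlapping a KillZVolume calls BallKill, then destroys the ball.
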(event `self.ReceiveActorBeginOverlap`
  (params (OtherActor :type "Actor Object Reference"))
  (cast `KillZVolume` OtherActor)
  (`self.BallKill`)
  (`self.K2_DestroyActor`))

(event `self.ReceiveTick`
  (params (DeltaSeconds :type "Float (single-precision)"))
  (bind _sweephitresult (`self.K2_AddActorWorldOffset` (* DeltaSeconds (`self.Direction`) (`self.Speed`)) true))
  (bind (_bblockinghit _binitialoverlap _time _distance _location _impactpoint _normal) (`GameplayStatics.BreakHitResult` _sweephitresult))
  (if _bblockinghit
    (set `self.Direction` (`KismetMathLibrary.GetReflectionVector` (`self.Direction`) _normal))))

(fn `UserConstructionScript`)