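; BP_BoxSpawner builds a grid of destructible blocks at BeginPlay, offset from its root location.
; Every fifth row and column, plus the last X row, gets a two-hit block, and the rest get one-hit boxes.
; It stores each spawned block in Blocks and relays its destruction through its own BlockDestroyed dispatcher with an enum identifying the block type.
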(event `self.ReceiveBeginPlay`
  (bind _offset (`self.Offset`))
  (bind _blocks (`self.Blocks`))
  (for _index (range (+ (`self.X_Blocks_Count`) 1))
    (for _index_2 (range (+ (`self.Y_Blocks_Count`) 1))
      (if (or (== (mod _index 5) 0) (== (mod _index_2 5) 0) (== _index (`self.X_Blocks_Count`)))
        (bind _returnvalue_location (`KismetMathLibrary.BreakTransform` (`KismetMathLibrary.MakeTransform` (`KismetMathLibrary.MakeVector` (`KismetMathLibrary.Conv_IntToDouble` (* _index _offset)) (`KismetMathLibrary.Conv_IntToDouble` (* _index_2 _offset)) 100.0))))
        (bind _returnvalue (+ _returnvalue_location (`SceneComponent.K2_GetComponentLocation` (`self.DefaultSceneRoot`))))
        (bind _returnvalue_2 (`|SpawnActorFromClass` "/Game/Actors/BP_TwoHits.BP_TwoHits_C" (`KismetMathLibrary.MakeTransform` _returnvalue) "AlwaysSpawn" "MultiplyWithRoot" null null))
        (add `/Game/Actors/BP_MasterBox.BlockDestroyed` _returnvalue_2 (delegate `TwoHitsBlockDestroyed`))
        (`KismetArrayLibrary.Array_Add` _blocks _returnvalue_2)
        (else
          (bind _returnvalue_3 (`|SpawnActorFromClass` "/Game/Actors/BP_OneHitBox.BP_OneHitBox_C" (`KismetMathLibrary.MakeTransform` _returnvalue) "AlwaysSpawn" "MultiplyWithRoot" null null))
          (add `/Game/Actors/BP_MasterBox.BlockDestroyed` _returnvalue_3 (delegate `OneHitBlockDestroyed`))
          (`KismetArrayLibrary.Array_Add` _blocks _returnvalue_3))))))

(event `TwoHitsBlockDestroyed`
  (`self.BlockDestroyed` "NewEnumerator1"))

(event `OneHitBlockDestroyed`
  (`self.BlockDestroyed` "NewEnumerator0"))

(fn `UserConstructionScript`)